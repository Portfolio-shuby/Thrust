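; BP_Turret is an AI turret that detects pawns with PawnSensing and fires bursts of BP_Bullet2 at the player.
; Tick yaws the head and aims the cannon at the target, spawning bullets through a counter and short Delay, and drops sight beyond a set range.
; When idle, the head sweeps between alternating yaws on a timer.
; A widget health bar faces the camera, and DecreaseHealth subtracts fixed damage, destroying the turret at zero.
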(event `self.ReceiveBeginPlay`)

(event `self.PawnSensing.OnSeePawn`
  (params (Pawn :type "Pawn Object Reference"))
  (set `self.Target` Pawn)
  (set `self.isSeeing` true))

(event `self.ReceiveTick`
  (params (DeltaSeconds :type "Float (single-precision)"))
  (bind _headparent (`self.HeadParent`))
  (bind _healthbarwidget (`self.HealthBarWidget`))
  (set `self.Delta Seconds` DeltaSeconds)
  (bind _aswb_turret_health_bar (cast `/Game/Shuby/BT_AI/HealthBar/WB_TurretHealthBar` (`WidgetComponent.GetWidget` (`self.HealthBarWidget`))))
  (`ProgressBar.SetPercent` (`/Game/Shuby/BT_AI/HealthBar/WB_TurretHealthBar.HealthBar` _aswb_turret_health_bar) (/ (`self.Health`) 100.0))
  (`SceneComponent.K2_SetWorldRotation` _healthbarwidget (`KismetMathLibrary.FindLookAtRotation` (`SceneComponent.K2_GetComponentLocation` _healthbarwidget) (`SceneComponent.K2_GetComponentLocation` (`Actor.RootComponent` (`GameplayStatics.GetPlayerCameraManager` 0)))) false false)
  (if (`self.isSeeing`)
    (bind (_sm_v _a_v) (`self.GetTwoLocations` (`self.Target`) (`self.HeadParent`)))
    (if (>= (`KismetMathLibrary.VSize` (- _sm_v _a_v)) 1100.0)
      (set `self.isSeeing` false))
    (bind _asbp_player (cast `/Game/Siru/BP/BP_Player` (`self.Target`)))
    (bind _output_get (set `self.As BP Player` _asbp_player))
    (bind (_sm_v_2 _a_v_2) (`self.GetTwoLocations` _output_get (`self.HeadParent`)))
    (bind (_returnvalue_roll _returnvalue_pitch _returnvalue_yaw) (`KismetMathLibrary.BreakRotator` (`KismetMathLibrary.FindLookAtRotation` _sm_v_2 _a_v_2)))
    (`SceneComponent.K2_SetWorldRotation` (`self.HeadParent`) (`KismetMathLibrary.MakeRotator` _returnvalue_roll 0.0 _returnvalue_yaw) false false)
    (bind (_sm_v_3 _a_v_3) (`self.GetTwoLocations` (`self.As BP Player`) (`self.CannonParent`)))
    (`SceneComponent.K2_SetWorldRotation` (`self.CannonParent`) (`KismetMathLibrary.FindLookAtRotation` _sm_v_3 _a_v_3) false false)
    (if (<= (`self.BulletTripple`) 2)
      (`KismetSystemLibrary.Delay` 0.05)
      (`|SpawnActorFromClass` "/Game/Shuby/BT_AI/Turret/BP_Bullet2.BP_Bullet2_C" (`SceneComponent.K2_GetComponentToWorld` (`self.Arrow`)) "Undefined" "MultiplyWithRoot" null null))
    (set `self.BulletTripple` (+ (`self.BulletTripple`) 1))
    (if (> (`self.BulletTripple`) 23)
      (set `self.BulletTripple` 0))
    (else
      (set `self.Time` (+ (`self.Time`) (`self.Delta Seconds`)))
      (if (>= (`self.Time`) 1.6)
        (set `self.Time` 0.0)
        (`KismetSystemLibrary.MoveComponentTo` _headparent (`SceneComponent.RelativeLocation` _headparent) (`KismetMathLibrary.MakeRotator` 0.0 0.0 (`self.ZAxis`)) false false 1.0)
        (set `self.ZAxis` (* (`self.ZAxis`) -1.0))))))

(fn `DecreaseHealth`
  (bind _aswb_turret_health_bar (cast `/Game/Shuby/BT_AI/HealthBar/WB_TurretHealthBar` (`WidgetComponent.GetWidget` (`self.HealthBarWidget`))))
  (bind _output_get (set `self.Health` (- (`self.Health`) 10.0)))
  (`ProgressBar.SetPercent` (`/Game/Shuby/BT_AI/HealthBar/WB_TurretHealthBar.HealthBar` _aswb_turret_health_bar) (/ _output_get 100.0))
  (if (<= (`self.Health`) 0.0)
    (`self.K2_DestroyActor`)))

(fn `GetTwoLocations`
  (params (A :type "Actor Object Reference") (SM :type "StaticMeshComponent Object Reference"))
  (returns (SM_V :type "Vector Structure") (A_V :type "Vector Structure"))
  (return (`SceneComponent.K2_GetComponentLocation` SM) (`self.K2_GetActorLocation` A)))

(fn `UserConstructionScript`)